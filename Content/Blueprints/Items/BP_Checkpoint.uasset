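; BP_Checkpoint is a checkpoint that sets where the player respawns.
; When BP_Player2 overlaps its Box, it flags the player as having a checkpoint and stores the RespawnPoint world transform on that player.
; The HaloFX particle color parameter starts yellow-green from the construction script and switches to a blue tint on activation, showing the checkpoint is reached.
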(event `self.box.OnComponentBeginOverlap`
  (params (OverlappedComponent :type "PrimitiveComponent Object Reference") (OtherActor :type "Actor Object Reference") (OtherComp :type "PrimitiveComponent Object Reference") (OtherBodyIndex :type Integer) (bFromSweep :type Boolean) (SweepResult :type "HitResult Structure (by ref)"))
  (bind _asbp_player_2 (cast `/Game/Blueprints/Player/BP_Player2` OtherActor))
  (set `/Game/Blueprints/Player/BP_Player2.hasCheckpoint` true _asbp_player_2)
  (set `/Game/Blueprints/Player/BP_Player2.CheckpointTransform` (`SceneComponent.K2_GetComponentToWorld` (`self.RespawnPoint`)) _asbp_player_2)
  (`NiagaraComponent.SetVariableLinearColor` (`self.HaloFX`) "User.ParticleColor" (make `LinearColor` 40.0 40.0 100.0)))

(fn `UserConstructionScript`
  (`NiagaraComponent.SetVariableLinearColor` (`self.HaloFX`) "User.ParticleColor" (make `LinearColor` 40.0 100.0)))